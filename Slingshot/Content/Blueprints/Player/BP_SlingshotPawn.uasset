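; BP_SlingshotPawn is the player's slingshot pawn, moved sideways and tilted by axis input.
; The Horizontal axis feeds FloatingPawnMovement along world X; at or beyond XBounds on either side, input is replaced by a constant push toward negative X.
; The Pitch axis adds local pitch rotation, with no effective limit because its guard conditions are hardcoded false.
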(event EventBeginPlay)

(event Input|AxisEvents|InputAxisHorizontal
  (params (AxisValue :type Float%20%28single-precision%29))
  ;[1 1 1] Movement
  (Class|PawnMovementComponent|AddInputVector (Variables|Default|GetFloatingPawnMovement) (Math|Vector|MakeVector (select (>= (Math|Float|Absolute(Float) (.X (Math|Vector|BreakVector (Transformation|GetActorLocation)))) (Variables|Default|GetXBounds)) -1.0 AxisValue) 0.0 0.0) false))

(event Input|AxisEvents|InputAxisPitch
  (params (AxisValue :type Float%20%28single-precision%29))
  ;[1 1 1] Rotation
  (Transformation|AddActorLocalRotation (Math|Rotator|MakeRotator 0.0 (select (or false false) 0.0 AxisValue) 0.0) false false))

(fn ConstructionScript)